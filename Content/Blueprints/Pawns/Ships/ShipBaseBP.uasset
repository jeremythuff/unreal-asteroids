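; Base ship pawn Blueprint that turns thrust, yaw and fire input into ship movement and a placeholder firing action.
; Each Tick, a sequence runs three macros that check the input values for non-zero, feeding the Thrust, Rotate and Fire functions.
; Thrust scales input into the forward thruster's strength, while Rotate adds world yaw to the mesh without delta-time scaling.
; Fire only prints a debug string at full input.
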(event EventTick
  (params (DeltaSeconds :type Float%20%28single-precision%29))
  ;[1 1 1] Tick Events
  (Utilities|FlowControl|Sequence
    (:then_0
      (bind _thrust (Utilities|IfThrusting)
        (:Thrusting
          _)
        (:Not%20Trusting
          _))
      (CallFunction|Thrust _thrust))
    (:then_1
      (bind _rotation (Utilities|IfRotating)
        (:Rotating
          (CallFunction|Rotate _rotation))))
    (:then_2
      (Utilities|IfFiring
        (:Firing
          (CallFunction|Fire))))))

(fn ConstructionScript)

(fn Fire
  (if (>= (Input|AxisValues|GetFire) 1.0)
    (Development|PrintString "Fire")))

(fn Rotate
  (params (Rotation :type Float%20%28single-precision%29))
  (Transformation|AddWorldRotation (Variables|Default|GetShipBaseMesh) (Math|Rotator|MakeRotator 0.0 0.0 Rotation) false false))

(fn Thrust
  (params (Thrust :type Float%20%28single-precision%29))
  (Variables|/Script/Engine.PhysicsThrusterComponent|SetThrustStrength (Variables|Default|GetForeward%20Thruster) (* Thrust 1e+03)))